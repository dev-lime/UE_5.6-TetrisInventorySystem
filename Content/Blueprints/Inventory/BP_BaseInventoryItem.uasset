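; BP_BaseInventoryItem is the base world pickup actor for a grid-based inventory system.
; On BeginPlay it builds a default item object from its item info, size and equipment class if none is set, allowing rotation only for non-square sizes.
; Interacting tries to add that object to the inventory, then plays a sound, adds weight and destroys the actor, or prints an overflow warning.
; Outline highlighting toggles the mesh's custom depth.
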(event Custom|EnableOutline
  (Rendering|SetRenderCustomDepth (Variables|Default|GetStaticMesh) true))

(event Custom|DisableOutline
  (Rendering|SetRenderCustomDepth (Variables|Default|GetStaticMesh) false))

(event EventInteract
  (params (InventoryComponent :type BPC%20Inventory%20Object%20Reference))
  (bind _added (Default|TryAddItem InventoryComponent (Variables|Private|GetItemObject) false))
  (if _added
    (Audio|PlaySound2D (Variables|Default|GetTakeItemSound) 1.0 1.0 0.0 0 0)
    (Default|AddInventoryWeight InventoryComponent (Variables|Private|GetItemObject))
    (Actor|DestroyActor)
    (else
      (Development|PrintString "Inventory is overflowing" true false "(R=1.000000,G=0.000000,B=0.000000,A=1.000000)" 3.0 "InventoryOverflowing"))))

(event EventBeginPlay
  (Utilities|IsValid (Variables|Private|GetItemObject)
    (:Is%20Not%20Valid
      (bind _itemobject (CallFunction|GetDefaultItemObject))
      (Variables|Private|SetItemObject _itemobject))))

(fn ConstructionScript)

(fn GetDefaultItemObject
  (bind _self self)
  (bind _itemsize (Variables|Default|GetItemSize))
  (bind _iteminfo (Variables|Default|GetItemInfo))
  (bind _returnvalue (Math|Float|Truncate (.y _itemsize)))
  (bind _returnvalue_2 (Math|Float|Truncate (.x _itemsize)))
  (bind _returnvalue_3 (Game|ConstructObjectfromClass _self "/Game/Blueprints/Inventory/BP_BaseItemObject.BP_BaseItemObject_C" (Variables|Default|GetItemInfo) (Utilities|Struct|MakeIntPoint _returnvalue_2 _returnvalue) (Utilities|GetClass _self) (!= _returnvalue_2 _returnvalue) (.defaultamount _iteminfo) (.defaultcondition _iteminfo) (.defaultweight _iteminfo) (Variables|Default|GetEquipment%20Class)))
  (return _returnvalue_3))

(fn GetOutline
  (return (Variables|/Script/Engine.PrimitiveComponent|GetbRenderCustomDepth (Variables|Default|GetStaticMesh))))