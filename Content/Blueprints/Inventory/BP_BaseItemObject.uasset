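; BP_BaseItemObject is the base inventory item object, holding an item's info, classes, stack amount, condition, weight and two-axis size.
; Rotation, when allowed, swaps the reported dimensions, and setters cap amount at the item's maximum and reset over-default condition to 100.
; UseItem applies the item's stats through the player's state component, decrements the stack and weights, and removes the item from the player's inventory component when empty.
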(fn GetDimension
  (bind _dimension (Variables|Default|GetDimension))
  (if (Variables|Default|GetIsRotate)
    (return (Utilities|Struct|MakeIntPoint (.y _dimension) (.x _dimension)))
    (else
      (return (Variables|Default|GetDimension)))))

(fn GetItemClass
  (return (Variables|Default|GetItemClass)))

(fn GetRotate
  (return (Variables|Default|GetIsRotate)))

(fn GetAmount
  (return (Variables|Default|GetAmount)))

(fn GetItemInfo
  (return (Variables|Default|GetItemInfo)))

(fn SetRotate
  (if (Variables|Default|GetCanRotate)
    (Variables|Default|SetIsRotate (not (Variables|Default|GetIsRotate)))))

(fn SetAmount
  (params (Amount :type Integer))
  (Utilities|FlowControl|Sequence
    (:then_0
      (if (<= Amount (.maxamount (Variables|Default|GetItemInfo)))
        (Variables|Default|SetAmount Amount)
        (else
          (Variables|Default|SetAmount (.maxamount (Variables|Default|GetItemInfo))))))
    (:then_1
      (return (Variables|Default|GetAmount)))))

(fn GetCondition
  (return (Variables|Default|GetCondition)))

(fn SetCondition
  (params (Condition :type Float%20%28double-precision%29))
  (Utilities|FlowControl|Sequence
    (:then_0
      (if (<= (Variables|Default|GetCondition) (.defaultcondition (GetItemInfo|GetItemInfo)))
        (Variables|Default|SetCondition Condition)
        (else
          (Variables|Default|SetCondition 1e+02))))
    (:then_1
      (return self))))

(fn GetWeight
  (return (Variables|Default|GetWeight)))

(fn GetEquipmentClass
  (return (Variables|Default|GetEquipmentClass)))

(fn SetWeight
  (params (Weight :type Float%20%28double-precision%29))
  (Utilities|FlowControl|Sequence
    (:then_0
      (Variables|Default|SetWeight Weight))
    (:then_1
      (return self))))

(fn UseItem
  (params (Player :type BP%20Character%20Object%20Reference))
  (bind _self self)
  (bind _bpc_inventory (Variables|/Game/Character/Blueprints/BP_Character.BP_Character_C|GetBPC_Inventory Player))
  (bind _iteminfo (Variables|Default|GetItemInfo))
  (Default|AddPlayerState (Variables|/Game/Character/Blueprints/BP_Character.BP_Character_C|GetBPC_PlayerState Player) (.playerstats _iteminfo))
  (bind _itemamount (SetItemInfo|SetAmount (- (GetItemInfo|GetAmount) 1)))
  (Variables|/Game/Blueprints/Inventory/BPC_Inventory.BPC_Inventory_C|SetInventoryWeight _bpc_inventory (- (Variables|/Game/Blueprints/Inventory/BPC_Inventory.BPC_Inventory_C|GetInventoryWeight _bpc_inventory) (.defaultweight _iteminfo)))
  (if (<= _itemamount 0)
    (Default|RemoveItem _bpc_inventory _self)
    (else
      (SetItemInfo|SetWeight _self (- (GetItemInfo|GetWeight) (.defaultweight _iteminfo))))))