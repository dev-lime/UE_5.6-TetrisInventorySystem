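; Equipment component that puts inventory items into the player's melee, secondary and primary weapon slots.
; AddToEquipSlot reads the item's equipment class defaults to match Melee or Firearms to a slot number, then spawns the weapon through that slot's ChildActorComponent.
; An occupied slot goes through SwitchEquip, which swaps only if the old item fits back into the inventory, though the slot variable takes the new item either way.
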(event EventBeginPlay)

(event EventTick
  (params (DeltaSeconds :type Float%20%28single-precision%29)))

(fn Initialization
  (params (Player :type BP%20Character%20Object%20Reference))
  (Variables|Default|SetPlayer Player))

(fn AddtoEquipSlot
  (params (EquipItem :type BP%20Base%20Item%20Object%20Object%20Reference) (EquipType :type EquipType_Enum%20Enum :default "NewEnumerator2") (SlotNumber :type SlotNumber_Enum%20Enum :default "NewEnumerator0"))
  (bind _equipmentclass (Default|GetEquipmentClass EquipItem))
  (if (Utilities|IsValidClass _equipmentclass)
    (Utilities|FlowControl|Sequence
      (:then_0
        (switch Utilities|FlowControl|Switch|SwitchonEquipType_Enum (Utilities|GetClassDefaults _equipmentclass)
          (:NewEnumerator2
            (switch Utilities|FlowControl|Switch|SwitchonSlotNumber_Enum SlotNumber
              (:NewEnumerator0
                (Utilities|IsValid (Variables|Default|GetMeleeSlot)
                  (:Is%20Valid
                    (bind _added (CallFunction|SwitchEquip EquipItem (Variables|Default|GetMeleeSlot) EquipType SlotNumber))
                    (Variables|Default|SetMeleeSlot EquipItem)
                    (return _added))
                  (:Is%20Not%20Valid
                    (ChildActorComponent|SetChildActorClass (Variables|/Game/Character/Blueprints/BP_Character.BP_Character_C|GetMeleeWeapon (Variables|Default|GetPlayer)) (Default|GetEquipmentClass EquipItem))
                    (Variables|Default|SetMeleeSlot EquipItem)
                    (return true))))))
          (:NewEnumerator4
            (switch Utilities|FlowControl|Switch|SwitchonSlotNumber_Enum SlotNumber
              (:NewEnumerator1
                (Utilities|IsValid (Variables|Default|GetSecondarySlot)
                  (:Is%20Valid
                    (bind _added_2 (CallFunction|SwitchEquip EquipItem (Variables|Default|GetSecondarySlot) EquipType SlotNumber))
                    (Variables|Default|SetSecondarySlot EquipItem)
                    (return _added_2))
                  (:Is%20Not%20Valid
                    (ChildActorComponent|SetChildActorClass (Variables|/Game/Character/Blueprints/BP_Character.BP_Character_C|GetSecondaryWeapon (Variables|Default|GetPlayer)) (Default|GetEquipmentClass EquipItem))
                    (Variables|Default|SetSecondarySlot EquipItem)
                    (return true))))
              (:NewEnumerator2
                (Utilities|IsValid (Variables|Default|GetPrimarySlot)
                  (:Is%20Valid
                    (bind _added_3 (CallFunction|SwitchEquip EquipItem (Variables|Default|GetPrimarySlot) EquipType SlotNumber))
                    (Variables|Default|SetPrimarySlot EquipItem)
                    (return _added_3))
                  (:Is%20Not%20Valid
                    (ChildActorComponent|SetChildActorClass (Variables|/Game/Character/Blueprints/BP_Character.BP_Character_C|GetPrimaryWeapon (Variables|Default|GetPlayer)) (Default|GetEquipmentClass EquipItem))
                    (Variables|Default|SetPrimarySlot EquipItem)
                    (return true))))))))
      (:then_1
        (return false)))))

(fn RemoveEquip
  (params (EquipItem :type BP%20Base%20Item%20Object%20Object%20Reference) (SlotType :type EquipType_Enum%20Enum :default "NewEnumerator2") (SlotNumber :type SlotNumber_Enum%20Enum :default "NewEnumerator0"))
  (bind _player (Variables|Default|GetPlayer))
  (bind _equipmentclass (Default|GetEquipmentClass EquipItem))
  (if (Utilities|IsValidClass _equipmentclass)
    (Utilities|FlowControl|Sequence
      (:then_0
        (switch Utilities|FlowControl|Switch|SwitchonEquipType_Enum (Utilities|GetClassDefaults _equipmentclass)
          (:NewEnumerator2
            (switch Utilities|FlowControl|Switch|SwitchonSlotNumber_Enum SlotNumber
              (:NewEnumerator0
                (ChildActorComponent|SetChildActorClass (Variables|/Game/Character/Blueprints/BP_Character.BP_Character_C|GetMeleeWeapon _player) 0)
                (Variables|Default|SetMeleeSlot 0))))
          (:NewEnumerator4
            (switch Utilities|FlowControl|Switch|SwitchonSlotNumber_Enum SlotNumber
              (:NewEnumerator1
                (ChildActorComponent|SetChildActorClass (Variables|/Game/Character/Blueprints/BP_Character.BP_Character_C|GetSecondaryWeapon _player) 0)
                (Variables|Default|SetSecondarySlot 0))
              (:NewEnumerator2
                (ChildActorComponent|SetChildActorClass (Variables|/Game/Character/Blueprints/BP_Character.BP_Character_C|GetPrimaryWeapon _player) 0)
                (Variables|Default|SetPrimarySlot 0)))))))))

(fn SwitchEquip
  (params (NewItemObject :type BP%20Base%20Item%20Object%20Object%20Reference) (OldItemObject :type BP%20Base%20Item%20Object%20Object%20Reference) (EquipType :type EquipType_Enum%20Enum :default "NewEnumerator2") (SlotNumber :type SlotNumber_Enum%20Enum :default "NewEnumerator0"))
  (bind _added (Default|TryAddItem (Variables|/Game/Character/Blueprints/BP_Character.BP_Character_C|GetBPC_Inventory (Variables|Default|GetPlayer)) OldItemObject false))
  (if _added
    (CallFunction|RemoveEquip OldItemObject EquipType SlotNumber)
    (bind _added_2 (CallFunction|AddtoEquipSlot NewItemObject EquipType SlotNumber))
    (return _added_2)
    (else
      (return false))))