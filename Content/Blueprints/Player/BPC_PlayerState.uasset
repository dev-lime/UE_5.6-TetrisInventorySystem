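; Player component that tracks survival stats (health, hunger and thirst) in a PlayerState struct.
; Tick drains hunger and thirst over time at fixed rates, with thirst falling faster, and leaves health unchanged.
; AddPlayerState adds a struct of deltas to the current values.
; Both paths then call CheckPlayerState, which clamps each stat to the 0–100 range.
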(event EventBeginPlay)

(event EventTick
  (params (DeltaSeconds :type Float%20%28single-precision%29))
  (Variables|Default|SetPlayerState (Utilities|Struct|MakePlayerState_Structure (.health (Variables|Default|GetPlayerState)) (- (.hunger (Variables|Default|GetPlayerState)) (* DeltaSeconds 0.6)) (- (.thirst (Variables|Default|GetPlayerState)) (* DeltaSeconds 0.8))))
  (CallFunction|CheckPlayerState))

(fn AddPlayerState
  (params (HealthToAdd :type Player%20State%20Structure%20Structure))
  (Variables|Default|SetPlayerState (Utilities|Struct|MakePlayerState_Structure (+ (.health HealthToAdd) (.health (Variables|Default|GetPlayerState))) (+ (.hunger HealthToAdd) (.hunger (Variables|Default|GetPlayerState))) (+ (.thirst HealthToAdd) (.thirst (Variables|Default|GetPlayerState)))))
  (CallFunction|CheckPlayerState))

(fn CheckPlayerState
  (bind _playerstate (Variables|Default|GetPlayerState))
  (bind _playerstate_2 (Variables|Default|GetPlayerState))
  (bind _playerstate_3 (Variables|Default|GetPlayerState))
  (bind _playerstate_4 (Variables|Default|GetPlayerState))
  (Utilities|FlowControl|Sequence
    (:then_0
      (if (< (.health _playerstate) 0.0)
        (Utilities|Struct|SetmembersinPlayerState_Structure _playerstate_3 0.0)
        (elif (> (.health _playerstate) 1e+02)
          (Utilities|Struct|SetmembersinPlayerState_Structure _playerstate_3 1e+02))))
    (:then_1
      (if (< (.hunger _playerstate) 0.0)
        (Utilities|Struct|SetmembersinPlayerState_Structure _playerstate_4 0.0)
        (elif (> (.hunger _playerstate) 1e+02)
          (Utilities|Struct|SetmembersinPlayerState_Structure _playerstate_4 1e+02))))
    (:then_2
      (if (< (.thirst _playerstate) 0.0)
        (Utilities|Struct|SetmembersinPlayerState_Structure _playerstate_2 0.0)
        (elif (> (.thirst _playerstate) 1e+02)
          (Utilities|Struct|SetmembersinPlayerState_Structure _playerstate_2 1e+02))))))